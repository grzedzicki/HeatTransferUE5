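; BP_NodeOwner manages the 3D node grid of a heat simulation and links it to the UI.
; On BeginPlay it reads the grid size from the game instance, spawns BP_Node actors, the main widget and BP_ThreadActor.
; The thread actor handles calculation steps, history, reset and saving, while looping timers drive automatic stepping and rewinding.
; It also controls node layout and appearance, pause/load menus, and random temperatures for the main-menu visualization.
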(event Custom|Talk
  (Default|TalktoInstance (Variables|Default|GetThread%20Reference)))

(event Custom|AutoCalculateDelay
  (bind _returnvalue (Game|GetPlayerController 0))
  (bind _asbp_player_controller (Utilities|Casting|CastToBP_PlayerController _returnvalue))
  (if (Variables|/Game/FirstPerson/Blueprints/BP_PlayerController.BP_PlayerController_C|GetShouldBlock? _asbp_player_controller)
    (Development|PrintString "Blocked")
    (else
      (Variables|/Game/FirstPerson/Blueprints/BP_PlayerController.BP_PlayerController_C|SetIsAuto?ThenBlock _asbp_player_controller true)
      (Utilities|Time|SetTimerbyFunctionName 0 "Auto Calculate" 3.0 true))))

(event Custom|StopAutoCalculate
  (bind _returnvalue (Game|GetPlayerController 0))
  (bind _asbp_player_controller (Utilities|Casting|CastToBP_PlayerController _returnvalue))
  (if (Variables|/Game/FirstPerson/Blueprints/BP_PlayerController.BP_PlayerController_C|GetShouldBlock? _asbp_player_controller)
    (Development|PrintString "Blocked")
    (else
      (Variables|/Game/FirstPerson/Blueprints/BP_PlayerController.BP_PlayerController_C|SetIsAuto?ThenBlock _asbp_player_controller false)
      (Utilities|Time|ClearTimerbyFunctionName 0 "Auto Calculate"))))

(event Custom|AutoReturnPreviousCalculations
  (bind _returnvalue (Game|GetPlayerController 0))
  (bind _asbp_player_controller (Utilities|Casting|CastToBP_PlayerController _returnvalue))
  (bind _shouldblock_ (Variables|/Game/FirstPerson/Blueprints/BP_PlayerController.BP_PlayerController_C|GetShouldBlock? _asbp_player_controller))
  (Utilities|FlowControl|FlipFlop
    (:A
      (if _shouldblock_
        (Development|PrintString "Blocked")
        (else
          (Utilities|Time|SetTimerbyFunctionName 0 "Return Previous Step" 1.0 true))))
    (:B
      (if _shouldblock_
        (Development|PrintString "Blocked")
        (else
          (Utilities|Time|ClearTimerbyFunctionName 0 "Return Previous Step"))))))

(event Custom|DisplayUpdateInfo
  (bind _widget_reference (Variables|Default|GetWidget%20Reference))
  (bind _textblock_21 (Variables|/Game/FirstPerson/Blueprints/BP_MainWidget.BP_MainWidget_C|GetTextBlock_21 _widget_reference))
  (Utilities|FlowControl|Delay 1.0)
  (Widget|SetVisibility _textblock_21 "Visible")
  (Utilities|FlowControl|Delay 1.0)
  (Widget|SetVisibility _textblock_21 "Hidden"))

(event EventBeginPlay
  (bind _returnvalue (Game|GetPlayerController 0))
  ;[0 0 0] Tworzenie BP_NodeOwner
  (Variables|/Game/FirstPerson/Blueprints/BP_HeatGameInstance.BP_HeatGameInstance_C|SetNode%20Owner%20Reference (.AsBP%20Heat%20Game%20Instance (Utilities|Casting|CastToBP_HeatGameInstance (Game|GetGameInstance))) self)
  (Variables|/Game/FirstPerson/Blueprints/BP_PlayerController.BP_PlayerController_C|SetMain%20Menu? (.AsBP%20Player%20Controller (Utilities|Casting|CastToBP_PlayerController _returnvalue)) false)
  (Input|SetInputModeGameOnly _returnvalue)
  (Utilities|FlowControl|Delay 0.001)
  (bind _asbp_player_controller (Utilities|Casting|CastToBP_PlayerController (Game|GetPlayerController 0))
    (:then
      (Default|SetNodeOwnerReference _asbp_player_controller self)
      ;[0 0 0] Tworzenie tablicy BP_Node, widgetu, wywołanie BP_ThreadActor, pobranie informacji na temat iteracji
      (CallFunction|CreateArrayOfNodes)
      (CallFunction|CreateWidget)
      (CallFunction|CreateThread)
      (CallFunction|GetIterations)
      (CallFunction|SetWidgetInfo))
    (:CastFailed
      (Development|PrintString "Cast Failed"))))

(fn ConstructionScript)

(fn GetGridSize
  ;[0 0 0] Przekazanie wielkości siatki
  (bind _asheat_game_instance (Utilities|Casting|CastToHeatGameInstance (Game|GetGameInstance)))
  (return (Variables|/Script/CleanHeatTransfer.HeatGameInstance|GetGrid_Size_1 _asheat_game_instance) (Variables|/Script/CleanHeatTransfer.HeatGameInstance|GetGrid_Size_2 _asheat_game_instance) (Variables|/Script/CleanHeatTransfer.HeatGameInstance|GetGrid_Size_3 _asheat_game_instance)))

(fn GetNodeStartingPostion
  (bind _returnvalue (Game|GetPlayerController 0))
  (bind _returnvalue_2 (+ 4.0 0.0))
  (bind _returnvalue_3 (Transformation|GetActorLocation _returnvalue))
  (bind _returnvalue_4 (+ (.x _returnvalue_3) -66.0))
  (bind _returnvalue_5 (+ (.y _returnvalue_3) -69.0))
  ;[0 0 0] Ustalenie początkowej pozycji węzłów
  (Variables|Default|SetInitial%20Position (Math|Vector|MakeVector _returnvalue_4 _returnvalue_5 _returnvalue_2))
  (return (Math|Vector|MakeVector _returnvalue_4 _returnvalue_5 _returnvalue_2)))

(fn CreateArrayOfNodes
  ;[0 0 0] Utworzenie tablicy węzłów
  (bind (_grid_size_1 _grid_size_2 _grid_size_3) (CallFunction|GetGridSize))
  (Variables|Default|SetGrid%20Size_1 _grid_size_1)
  (Variables|Default|SetGrid%20Size_2 _grid_size_2)
  (Variables|Default|SetGrid%20Size_3 _grid_size_3)
  (bind _node_starting_position (CallFunction|GetNodeStartingPostion))
  (LocalVariables|SetNode%20Starting%20Position _node_starting_position)
  (for _index (range 0 (- (* (Variables|Default|GetGrid%20Size_1) (Variables|Default|GetGrid%20Size_2) (Variables|Default|GetGrid%20Size_3)) 1))
    (bind _returnvalue (Game|SpawnActorfromClass "/Game/FirstPerson/Blueprints/BP_Node.BP_Node_C" (Math|Transform|MakeTransform (LocalVariables|GetNode%20Starting%20Position) "0, 0, 0" "0.100000,0.100000,0.100000") "Undefined" 0 0))
    (bind _output_get (LocalVariables|SetCurrent%20Node _returnvalue))
    (Variables|/Game/FirstPerson/Blueprints/BP_Node.BP_Node_C|SetId%20Node _output_get _index)
    (Default|ReferenceNodeOwner (LocalVariables|GetCurrent%20Node) self)
    (Utilities|Array|Add (Variables|Default|GetNodeArray) (LocalVariables|GetCurrent%20Node)))
  (Development|PrintString (Utilities|String|Append "Created " (Utilities|String|ToString(Integer) (* (Variables|Default|GetGrid%20Size_1) (Variables|Default|GetGrid%20Size_2) (Variables|Default|GetGrid%20Size_3))) " nodes!")))

(fn CreateWidget
  (bind _returnvalue (Game|GetGameInstance))
  (bind _asbp_heat_game_instance (Utilities|Casting|CastToBP_HeatGameInstance _returnvalue))
  (bind _sliderval (Variables|/Script/CleanHeatTransfer.HeatGameInstance|GetSliderVal _asbp_heat_game_instance))
  (bind _returnvalue_2 (Math|Conversions|ToFloat(Integer) _sliderval))
  ;[0 0 0] Na podstawie CheckoBoxów, jeśli siatka była wczytana z pliku to widget jest wywołany już w odpowiednim stanie
  (bind _returnvalue_3 (UserInterface|CreateWidget "/Game/FirstPerson/Blueprints/BP_MainWidget.BP_MainWidget_C"))
  (bind _output_get (Variables|Default|SetWidget%20Reference _returnvalue_3))
  (Variables|/Game/FirstPerson/Blueprints/BP_MainWidget.BP_MainWidget_C|SetNode%20Owner%20Reference _output_get self)
  (if (Variables|/Game/FirstPerson/Blueprints/BP_HeatGameInstance.BP_HeatGameInstance_C|GetNew? _asbp_heat_game_instance)
    _
    (else
      (if (Variables|/Script/CleanHeatTransfer.HeatGameInstance|GetLong_distance _asbp_heat_game_instance)
        (Class|Slider|SetMaxValue (Variables|/Game/FirstPerson/Blueprints/BP_MainWidget.BP_MainWidget_C|GetDistanceBetweenNodes _returnvalue_3) 3e+02))
      (Class|Slider|SetValue (Variables|/Game/FirstPerson/Blueprints/BP_MainWidget.BP_MainWidget_C|GetDistanceBetweenNodes _returnvalue_3) _returnvalue_2)
      (if (Variables|/Script/CleanHeatTransfer.HeatGameInstance|GetBig_size _asbp_heat_game_instance)
        (Class|Slider|SetMaxValue (Variables|/Game/FirstPerson/Blueprints/BP_MainWidget.BP_MainWidget_C|GetSizeOfNodes _returnvalue_3) 2.0))
      (Class|Slider|SetValue (Variables|/Game/FirstPerson/Blueprints/BP_MainWidget.BP_MainWidget_C|GetSizeOfNodes _returnvalue_3) (Variables|/Script/CleanHeatTransfer.HeatGameInstance|GetNode_size _asbp_heat_game_instance))
      (CallFunction|ChangeDistanceBetweenNodes (Math|Float|Truncate _returnvalue_2))))
  (if (not (Variables|/Game/FirstPerson/Blueprints/BP_HeatGameInstance.BP_HeatGameInstance_C|GetViz? _asbp_heat_game_instance))
    (UserInterface|Viewport|AddtoViewport (Variables|Default|GetWidget%20Reference) 0)))

(fn ChangeDistanceBetweenNodes
  (params (Distance :type Integer))
  (bind _returnvalue (Game|GetGameInstance))
  (bind _initial_position (Variables|Default|GetInitial%20Position))
  (bind _asbp_heat_game_instance (Utilities|Casting|CastToBP_HeatGameInstance _returnvalue))
  ;[0 0 0] Na podstawie rozmiarów siatki oraz wybranego odstępu między węzłami dopasowywana jest nowa pozycja
  (LocalVariables|SetDistance%20Between%20Nodes Distance)
  (for _array_element (Variables|Default|GetNodeArray)
    (LocalVariables|SetX%20Value (.x _initial_position))
    (LocalVariables|SetY%20Value (.y _initial_position))
    (LocalVariables|SetZ%20Value (.z _initial_position))
    (Transformation|SetActorLocation _array_element (Math|Vector|MakeVector (+ (LocalVariables|GetX%20Value) (* (* (Variables|/Script/CleanHeatTransfer.HeatGameInstance|GetDelta_x _asbp_heat_game_instance) (LocalVariables|GetX%20Iterator)) (LocalVariables|GetDistance%20Between%20Nodes))) (+ (LocalVariables|GetY%20Value) (* (* (Variables|/Script/CleanHeatTransfer.HeatGameInstance|GetDelta_y _asbp_heat_game_instance) (LocalVariables|GetY%20Iterator)) (LocalVariables|GetDistance%20Between%20Nodes))) (+ (LocalVariables|GetZ%20Value) (* (* (Variables|/Script/CleanHeatTransfer.HeatGameInstance|GetDelta_z _asbp_heat_game_instance) (LocalVariables|GetZ%20Iterator)) (LocalVariables|GetDistance%20Between%20Nodes)))) true false)
    (bind _result (Math|Integer|IncrementInt (LocalVariables|GetY%20Iterator))
      (:%20%20
        (if (== _result (Variables|Default|GetGrid%20Size_2))
          (LocalVariables|SetY%20Iterator 0)
          (Math|Integer|IncrementInt (LocalVariables|GetZ%20Iterator)
            (:%20%20
              (if (== (LocalVariables|GetZ%20Iterator) (Variables|Default|GetGrid%20Size_3))
                (LocalVariables|SetZ%20Iterator 0)
                (Math|Integer|IncrementInt (LocalVariables|GetX%20Iterator)
                  (:%20%20
                    (if (== (LocalVariables|GetX%20Iterator) (Variables|Default|GetGrid%20Size_1))
                      (LocalVariables|SetX%20Iterator 0))))))))))))

(fn CalculateNextStep
  ;[0 0 0] Wywołanie kolejnego kroku obliczeniowego
  (if (Variables|/Game/FirstPerson/Blueprints/BP_PlayerController.BP_PlayerController_C|GetShouldBlock? (.AsBP%20Player%20Controller (Utilities|Casting|CastToBP_PlayerController (Game|GetPlayerController 0))))
    (Development|PrintString "Blocked")
    (else
      (Default|CalculateNextStep (Variables|Default|GetThread%20Reference))
      (if (not (Variables|/Game/FirstPerson/Blueprints/BP_HeatGameInstance.BP_HeatGameInstance_C|GetViz? (.AsBP%20Heat%20Game%20Instance (Utilities|Casting|CastToBP_HeatGameInstance (Game|GetGameInstance)))))
        (CallFunction|GetIterations)))))

(fn CreateThread
  ;[0 0 0] Stworzenie klasy umożliwiającej wywołanie klasy obliczeniowej FRunnable
  (bind _returnvalue (Game|SpawnActorfromClass "/Game/FirstPerson/Blueprints/BP_ThreadActor.BP_ThreadActor_C" (Transformation|GetActorTransform (Game|GetPlayerController 0)) "Undefined" 0 0))
  (bind _output_get (Variables|Default|SetThread%20Reference _returnvalue))
  (Default|CreateThreadReference _output_get self (Variables|Default|GetGrid%20Size_1) false))

(fn ReturnPreviousStep
  (bind _thread_reference (Variables|Default|GetThread%20Reference))
  ;[0 0 0] Przywracanie poprzedniego kroku obliczeń
  (if (Variables|/Game/FirstPerson/Blueprints/BP_PlayerController.BP_PlayerController_C|GetShouldBlock? (.AsBP%20Player%20Controller (Utilities|Casting|CastToBP_PlayerController (Game|GetPlayerController 0))))
    (Development|PrintString "Blocked")
    (else
      (bind _previous_exist_ (Default|ReturnPreviousStep _thread_reference))
      (if _previous_exist_
        (Default|ReturnNewArray _thread_reference)
        (CallFunction|GetIterations)))))

(fn ResetAll
  ;[0 0 0] Usunięcie całej siatki
  (for _array_element (Variables|Default|GetNodeArray)
    (Variables|/Game/FirstPerson/Blueprints/BP_Node.BP_Node_C|SetTemperature _array_element 0.0)
    (Variables|/Game/FirstPerson/Blueprints/BP_Node.BP_Node_C|SetConstant%20Temperature _array_element false))
  (Default|ResetData (Variables|Default|GetThread%20Reference)))

(fn AddtoTemp
  ;[0 0 0] Dodanie obecnych zmian do tymczasowej mapy
  (for _array_element (Variables|Default|GetNodeArray)
    (Utilities|Array|Add (LocalVariables|GetHeat%20Array) (Variables|/Game/FirstPerson/Blueprints/BP_Node.BP_Node_C|GetTemperature _array_element))
    (Utilities|Array|Add (LocalVariables|GetBool%20Array) (Variables|/Game/FirstPerson/Blueprints/BP_Node.BP_Node_C|GetConstant%20Temperature _array_element)))
  (Default|SavetoTempMap (Variables|Default|GetThread%20Reference) (LocalVariables|GetHeat%20Array) (LocalVariables|GetBool%20Array)))

(fn Redo
  (Default|ReturnRedo (Variables|Default|GetThread%20Reference)))

(fn UpdateArray
  (for _array_element (Variables|Default|GetNodeArray)
    (Default|SetNewTemperaturefromTemp _array_element (Variables|/Game/FirstPerson/Blueprints/BP_Node.BP_Node_C|GetTemperature _array_element) (Variables|/Game/FirstPerson/Blueprints/BP_Node.BP_Node_C|GetConstant%20Temperature _array_element))))

(fn CreatePauseMenuWidget
  (params (Create? :type Boolean))
  (bind _returnvalue (Game|GetPlayerController 0))
  ;[0 0 0] Wywołanie/usunięcie widgetu menu pauzy
  (if Create?
    (Widget|SetVisibility (Variables|Default|GetWidget%20Reference) "Hidden")
    (bind _returnvalue_2 (UserInterface|CreateWidget "/Game/FirstPerson/Blueprints/BP_PauseMenu.BP_PauseMenu_C"))
    (UserInterface|Viewport|AddtoViewport _returnvalue_2 0)
    (Default|CreateNodeOwnerReference _returnvalue_2 self)
    (Variables|Default|SetPause%20Menu%20Widget%20Reference _returnvalue_2)
    (else
      (Widget|RemovefromParent (Variables|Default|GetPause%20Menu%20Widget%20Reference))
      (Widget|SetVisibility (Variables|Default|GetWidget%20Reference) "SelfHitTestInvisible")
      (Input|SetInputModeGameandUI _returnvalue 0 "DoNotLock" true)
      (Variables|/Game/FirstPerson/Blueprints/BP_PlayerController.BP_PlayerController_C|SetClicked (.AsBP%20Player%20Controller (Utilities|Casting|CastToBP_PlayerController _returnvalue)) false))))

(fn GetAllSavedGames
  ;[0 0 0] Wypisanie wykrytych plików  do widgetu
  (bind _returnvalue (Class|FileManager|GetAllSavedFiles))
  (if (not (Utilities|Array|IsEmpty _returnvalue))
    (bind _returnvalue_2 (UserInterface|CreateWidget "/Game/FirstPerson/Blueprints/BP_LoadWidget.BP_LoadWidget_C"))
    (Variables|Default|SetLoad%20Widget%20Reference _returnvalue_2)
    (Default|DisplaySavedGames _returnvalue_2 _returnvalue)
    (UserInterface|Viewport|AddtoViewport _returnvalue_2 0)
    (Widget|SetVisibility (Variables|Default|GetPause%20Menu%20Widget%20Reference) "Hidden")
    (Variables|/Game/FirstPerson/Blueprints/BP_LoadWidget.BP_LoadWidget_C|SetNode%20Owner%20Reference _returnvalue_2 self)))

(fn CloseLoadWidget
  (Widget|RemovefromParent (Variables|Default|GetLoad%20Widget%20Reference))
  (Widget|SetVisibility (Variables|Default|GetPause%20Menu%20Widget%20Reference) "Visible"))

(fn SaveDatatoFile
  (Class|ThreadActor|SaveDatatoFile (Variables|Default|GetThread%20Reference)))

(fn AutoRotateNodes
  (for _array_element (Variables|Default|GetNodeArray)
    (Default|AutoRotateNode _array_element)))

(fn AutoCalculate
  (CallFunction|CalculateNextStep))

(fn ReturnFurther
  (Default|ReturnFurtherTemp (Variables|Default|GetThread%20Reference))
  (CallFunction|GetIterations))

(fn ChangeNodesMaterial
  (params (Transparent? :type Boolean))
  ;[0 0 0] Zmiana materiału węzłów między przezroczystym a kolorem
  (if Transparent?
    (for _array_element (Variables|Default|GetNodeArray)
      (Rendering|Material|SetMaterial (Variables|/Game/FirstPerson/Blueprints/BP_Node.BP_Node_C|GetSphere _array_element) 0 (Variables|/Game/FirstPerson/Blueprints/BP_Node.BP_Node_C|GetTemperature%20Color%20Normal%20Material%20Instance _array_element))
      (Default|SetNodeColor _array_element false))
    (else
      (for _array_element_2 (Variables|Default|GetNodeArray)
        (Rendering|Material|SetMaterial (Variables|/Game/FirstPerson/Blueprints/BP_Node.BP_Node_C|GetSphere _array_element_2) 0 "/Game/Blueprints/Glass_Mat.Glass_Mat")))))

(fn ChangeNodesSize
  (params (NewSize :type Float%20%28double-precision%29))
  ;[0 0 0] Zmiana rozmiaru węzłów
  (for _array_element (Variables|Default|GetNodeArray)
    (Transformation|SetWorldScale3D (Variables|/Game/FirstPerson/Blueprints/BP_Node.BP_Node_C|GetSphere _array_element) (* (Variables|Default|GetWorld%20Scale) (/ NewSize 2)))))

(fn CloseLoadReOpenPause
  (Widget|SetVisibility (Variables|Default|GetPause%20Menu%20Widget%20Reference) "Visible")
  (Widget|RemovefromParent (Variables|Default|GetLoad%20Widget%20Reference)))

(fn TellNodestoCheckOverlap
  ;[0 0 0] Węzeł sprawdza czy nachodzi na ścianę
  (for _array_element (Variables|Default|GetNodeArray)
    (Default|CheckYourself _array_element))
  (CallFunction|AddtoTemp))

(fn Viz:SetRandomTemps
  (bind _nodearray (Variables|Default|GetNodeArray))
  (bind _random_element (Utilities|NewMacro0 _nodearray))
  ;[0 0 0] Wyświetlenie temperatur w menu głównym
  (for _index (range 0 50)
    (bind _output (CallFunction|RandomTMP _nodearray))
    (Utilities|IsValid _output
      (:Is%20Valid
        (Default|SetNewTemperature _random_element (Math|Random|RandomFloatinRange 5e+01 1e+02) true false false)
        (Variables|/Game/FirstPerson/Blueprints/BP_Node.BP_Node_C|SetShowTemperature? _random_element true)))))

(fn GetCurrentStep
  ;[0 0 0] Przywrócenie oryginalnego stanu siatki
  (if (Variables|/Game/FirstPerson/Blueprints/BP_PlayerController.BP_PlayerController_C|GetShouldBlock? (.AsBP%20Player%20Controller (Utilities|Casting|CastToBP_PlayerController (Game|GetPlayerController 0))))
    (Development|PrintString "Blocked")
    (else
      (Default|ReturnNewArray (Variables|Default|GetThread%20Reference)))))

(fn StartAnew
  ;[0 0 0] Wyczyszczenie wszelkich danych siatki
  (if (Variables|/Game/FirstPerson/Blueprints/BP_PlayerController.BP_PlayerController_C|GetShouldBlock? (.AsBP%20Player%20Controller (Utilities|Casting|CastToBP_PlayerController (Game|GetPlayerController 0))))
    (Development|PrintString "Blocked")
    (else
      (Default|ResetData (Variables|Default|GetThread%20Reference))
      (for _array_element (Variables|Default|GetNodeArray)
        (Default|SetNewTemperature _array_element 0.0 false true false))
      (CallFunction|GetIterations)
      (CallFunction|SetWidgetInfo))))

(fn StopAutoRotate
  ;[0 0 0] Zatrzymanie automatycznego obracania i wyświetlanie wartości temperatur
  (for _array_element (Variables|Default|GetNodeArray)
    (Default|StopAutoRotateNode _array_element)))

(fn ShowTextTemperatures
  (for _array_element (Variables|Default|GetNodeArray)
    (Default|ShowTextTemperature _array_element)))

(fn GetIterations
  (bind _thread_reference (Variables|Default|GetThread%20Reference))
  (bind _widget_reference (Variables|Default|GetWidget%20Reference))
  ;[0 0 0] Pobranie informacji o aktualnej iteracji i kroku czasowym
  (bind (_user_iterator _map_iterator _current_heat_array_iteration_value) (Default|ReturnIterations _thread_reference))
  (Default|UpdateIterations _widget_reference (Utilities|Text|ToText(Integer) _user_iterator) (Utilities|Text|ToText(Integer) _map_iterator) (Utilities|Text|ToText(Integer) _current_heat_array_iteration_value))
  (Class|ThreadActor|SumIterationsValues _thread_reference)
  (Rendering|Components|TextRender|SetText (Variables|/Game/FirstPerson/Blueprints/BP_MainWidget.BP_MainWidget_C|GetTextBlock_20 _widget_reference) (Utilities|Text|ToText(Integer) (Variables|/Script/CleanHeatTransfer.ThreadActor|GetSumIterations _thread_reference)))
  (CallFunction|DisplayUpdateInfo))

(fn SetWidgetInfo
  (bind _returnvalue (Game|GetGameInstance))
  (bind _widget_reference (Variables|Default|GetWidget%20Reference))
  (bind _asbp_heat_game_instance (Utilities|Casting|CastToBP_HeatGameInstance _returnvalue))
  ;[0 0 0] Ustalenie wyświetlanych wartości w widgecie
  (Rendering|Components|TextRender|SetText (Variables|/Game/FirstPerson/Blueprints/BP_MainWidget.BP_MainWidget_C|GetDistanceBoxX _widget_reference) (Utilities|Text|ToText(Float) (Variables|/Script/CleanHeatTransfer.HeatGameInstance|GetDelta_x _asbp_heat_game_instance) "HalfToEven"))
  (Rendering|Components|TextRender|SetText (Variables|/Game/FirstPerson/Blueprints/BP_MainWidget.BP_MainWidget_C|GetDistanceBoxY _widget_reference) (Utilities|Text|ToText(Float) (Variables|/Script/CleanHeatTransfer.HeatGameInstance|GetDelta_y _asbp_heat_game_instance) "HalfToEven"))
  (Rendering|Components|TextRender|SetText (Variables|/Game/FirstPerson/Blueprints/BP_MainWidget.BP_MainWidget_C|GetDistanceBoxZ _widget_reference) (Utilities|Text|ToText(Float) (Variables|/Script/CleanHeatTransfer.HeatGameInstance|GetDelta_z _asbp_heat_game_instance) "HalfToEven"))
  (Rendering|Components|TextRender|SetText (Variables|/Game/FirstPerson/Blueprints/BP_MainWidget.BP_MainWidget_C|GetTextBlock_14 _widget_reference) (Utilities|Text|ToText(Float) (Variables|/Script/CleanHeatTransfer.HeatGameInstance|GetDelta_t _asbp_heat_game_instance) "HalfToEven"))
  (Rendering|Components|TextRender|SetText (Variables|/Game/FirstPerson/Blueprints/BP_MainWidget.BP_MainWidget_C|GetTextBlock_16 _widget_reference) (Utilities|Text|ToText(Float) (Variables|/Script/CleanHeatTransfer.HeatGameInstance|GetAlpha _asbp_heat_game_instance) "HalfToEven")))

(fn RandomTMP
  (params (TargetArray :type Array%20of%20BP%20Node%20Object%20References))
  (bind _returnvalue (Utilities|Array|Length TargetArray))
  (bind _returnvalue_2 (Math|Random|RandomInteger _returnvalue))
  ;[0 0 0] Wybranie losowych węzłów i ustalenie na nich losowych temperatur
  (if (Utilities|Array|IsValidIndex TargetArray _returnvalue_2)
    (return (Utilities|Array|Get(acopy) TargetArray _returnvalue_2) _returnvalue_2)))